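; OSC_AUDIO receives a volume level and an on/off toggle over OSC and stores them as Volume and AudioToggle.
; Two matching collapsed graphs bind the "audio/volume" and "audio/toggle" addresses on the OSCAudio server and read each message's first float.
; Tick re-issues both bindings every frame and zeroes Volume while the toggle is off.
; Values are printed for debugging, and no sound is driven here.
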(event Custom|CustomEvent_Audio
  (params (AddressPattern :type OSC%20Address%20Structure%20%28by%20ref%29) (Message :type OSC%20Message%20Structure%20%28by%20ref%29) (IPAddress :type String) (Port :type Integer))
  (|OSCControl_Audio "audio/volume" (delegate Custom|CustomEvent_Audio) Message) ; enters at execute2
)

(event Custom|CustomEvent
  (params (AddressPattern :type OSC%20Address%20Structure%20%28by%20ref%29) (Message :type OSC%20Message%20Structure%20%28by%20ref%29) (IPAddress :type String) (Port :type Integer))
  (|OSCControl_Audio_2 "audio/toggle" (delegate Custom|CustomEvent) Message) ; enters at execute2
)

(event EventTick
  (params (DeltaSeconds :type Float%20%28single-precision%29))
  (Utilities|FlowControl|Sequence
    (:then_0
      (if (== (Variables|Default|GetAudio%20Toggle) true)
        (bind _output_get (Variables|Default|SetVolume (Variables|Default|GetVolume)))
        (Development|PrintString (Utilities|String|ToString(Float) _output_get) true true "(R=0.000000,G=0.660000,B=1.000000,A=1.000000)" _output_get)
        (else
          (Variables|Default|SetVolume 0.0))))
    (:then_1
      (Utilities|FlowControl|Sequence
        (:then_0
          (bind _value (|OSCControl_Audio "audio/volume" (delegate Custom|CustomEvent_Audio) (stale Custom|CustomEvent_Audio Message)))
          (bind _output_get_2 (Variables|Default|SetVolume _value))
          (Development|PrintString (Utilities|String|ToString(Float) _output_get_2) true false))
        (:then_1
          (bind _value_2 (|OSCControl_Audio_2 "audio/toggle" (delegate Custom|CustomEvent) (stale Custom|CustomEvent Message)))
          (if (== _value_2 1.0)
            _
            (else
              _))
          (bind _output_get_3 (Variables|Default|SetAudio%20Toggle (== _value_2 1.0)))
          (Development|PrintString (Utilities|String|ToString(Boolean) _output_get_3)))))))

(fn ConstructionScript)