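; OSC_SKY makes the sky and lighting react to audio volume from an OSCAudio reference.
; While AudioToggle is on, Tick maps volume to lower Mie absorption and brighter SunSky and separate directional lights.
; When the toggle is off, a DoOnce zeroes the volume and reapplies that mapping.
; Tick also binds a "scene1" OSC address handler every frame, whose extracted float goes unused.
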(event Custom|CustomEvent_Audio
  (params (AddressPattern :type OSC%20Address%20Structure%20%28by%20ref%29) (Message :type OSC%20Message%20Structure%20%28by%20ref%29) (IPAddress :type String) (Port :type Integer))
  (|OSCControl_Audio "scene1" (delegate Custom|CustomEvent_Audio) Message) ; enters at execute2
)

(event EventTick
  (params (DeltaSeconds :type Float%20%28single-precision%29))
  (bind _osc_audio (Variables|Default|GetOSC%20Audio))
  (bind _sunsky_reference (Variables|Default|GetSunSky%20Reference))
  (bind _audio_toggle (Variables|/Game/Blueprints/OSC_AUDIO.OSC_AUDIO_C|GetAudio%20Toggle _osc_audio))
  (Utilities|FlowControl|Sequence
    (:then_0
      (if _audio_toggle
        (Utilities|FlowControl|Sequence
          (:then_0
            (Variables|Default|SetVolume%20Reference (Variables|/Game/Blueprints/OSC_AUDIO.OSC_AUDIO_C|GetVolume _osc_audio)))
          (:then_1
            (goto _label Reset)))
        (else
          (Utilities|FlowControl|DoOnce _audio_toggle :!label _label
            (:Completed
              (Variables|Default|SetVolume%20Reference 0.0)))))
      (Utilities|FlowControl|Sequence
        (:then_0
          (Class|SkyAtmosphereComponent|SetMieAbsorptionScale (Variables|/SunPosition/SunSky.SunSky_C|GetSkyAtmosphere _sunsky_reference) (Math|Float|MapRangeClamped (Variables|Default|GetVolume%20Reference) 0.0 0.5 0.5 0.000444)))
        (:then_1
          (Rendering|Components|Light|SetIntensity (Variables|/SunPosition/SunSky.SunSky_C|GetDirectionalLight _sunsky_reference) (Math|Float|MapRangeClamped (Variables|Default|GetVolume%20Reference) 0.0 0.5 0.601217 15.0)))
        (:then_2
          (Rendering|Components|Light|SetIntensity (Variables|/Script/Engine.Light|GetLightComponent (Variables|Default|GetDirectionalLight%20Reference)) (Math|Float|MapRangeClamped (Variables|Default|GetVolume%20Reference) 0.0 0.5 2.0 1e+01)))))
    (:then_1
      (Utilities|FlowControl|Sequence
        (:then_0
          (|OSCControl_Audio "scene1" (delegate Custom|CustomEvent_Audio) (stale Custom|CustomEvent_Audio Message)))))))

(fn ConstructionScript)