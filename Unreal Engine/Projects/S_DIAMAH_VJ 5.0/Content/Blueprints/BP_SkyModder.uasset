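; Sky modder actor that makes scene lighting and atmosphere react to an audio volume value.
; While the volume reference's audio toggle is on, Tick copies its value and clamp-remaps it into Mie absorption, two directional light intensities and post-process intensity and vignette.
; Louder values brighten the lights, lower absorption and strengthen the vignette.
; When the toggle turns off, a DoOnce applies zero volume once, re-arming while audio is on.
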(event EventBeginPlay
  (Variables|Components|SetSkyAtmosphereReference (Actor|GetComponentbyClass (Variables|Default|GetSunSkyReference) "/Script/Engine.SkyAtmosphereComponent")))

(event Collision|EventActorBeginOverlap
  (params (OtherActor :type Actor%20Object%20Reference)))

(event EventTick
  (params (DeltaSeconds :type Float%20%28single-precision%29))
  (bind _volumereference (Variables|Default|GetVolumeReference))
  (bind _sunskyreference (Variables|Default|GetSunSkyReference))
  (bind _audiotoggle (Variables|/Game/Blueprints/captureLR.captureLR_C|GetAudioToggle _volumereference))
  (if _audiotoggle
    (Utilities|FlowControl|Sequence
      (:then_0
        (Variables|Default|SetVolume (Variables|/Game/Blueprints/captureLR.captureLR_C|GetVolumeValue _volumereference)))
      (:then_1
        (goto _label Reset)))
    (else
      (Utilities|FlowControl|DoOnce _audiotoggle :!label _label
        (:Completed
          (Variables|Default|SetVolume 0.0)))))
  (Utilities|FlowControl|Sequence
    (:then_0
      (Class|SkyAtmosphereComponent|SetMieAbsorptionScale (Variables|/SunPosition/SunSky.SunSky_C|GetSkyAtmosphere _sunskyreference) (Math|Float|MapRangeClamped (Variables|Default|GetVolume) 0.0 0.5 0.5 0.000444)))
    (:then_1
      (Rendering|Components|Light|SetIntensity (Variables|/SunPosition/SunSky.SunSky_C|GetDirectionalLight _sunskyreference) (Math|Float|MapRangeClamped (Variables|Default|GetVolume) 0.0 0.5 0.601217 15.0)))
    (:then_2
      (Rendering|Components|Light|SetIntensity (Variables|/Script/Engine.Light|GetLightComponent (Variables|Default|GetDirectionalLightReference)) (Math|Float|MapRangeClamped (Variables|Default|GetVolume) 0.0 0.5 2.0 1e+01)))
    (:then_3
      (Utilities|Struct|SetmembersinPostProcessSettings (Variables|/Script/Engine.PostProcessVolume|GetSettings (Variables|Default|GetPostProcessReference)) (Math|Float|MapRangeClamped (Variables|Default|GetVolume) 0.0 0.5 0.675 1e+01) (Math|Float|MapRangeClamped (Variables|Default|GetVolume) 0.0 0.5 0.0 1.5)))))

(fn ConstructionScript)