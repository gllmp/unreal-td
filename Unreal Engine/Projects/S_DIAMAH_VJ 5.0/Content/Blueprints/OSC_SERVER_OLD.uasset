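; OSC server actor that lets external messages drive a scene live on localhost port 7000.
; Addresses control a cube, lights, sky, post-processing, camera blends, level streaming and captureLR audio settings.
; BeginPlay creates the server and logs incoming messages; Tick re-binds every address each frame, or recreates the server if invalid.
; Repeated OSC Control subgraphs each bind an address to an event and extract the message value to apply.
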(event Custom|OnMsgReceived
  (params (Message :type OSC%20Message%20Structure%20%28by%20ref%29) (IPAddress :type String) (Port :type Integer))
  ;[1 1 1] Binding to Any Message
  (bind _returnvalue (Class|OSCManager|GetOSCMessageAddress Message))
  (bind _returnvalue_2 (Class|OSCManager|GetOSCAddressFullPath _returnvalue))
  (bind _value (Class|OSCManager|GetFloat Message))
  (Development|PrintString (Utilities|String|Append "Address: " _returnvalue_2 "/ " (Utilities|String|ToString(Float) _value)) false))

(event Custom|CustomEvent_10
  (params (AddressPattern :type OSC%20Address%20Structure%20%28by%20ref%29) (Message :type OSC%20Message%20Structure%20%28by%20ref%29) (IPAddress :type String) (Port :type Integer))
  (|OSCOSCControl_Cam_2_2 "scene1/camera/speed" (delegate Custom|CustomEvent_10) Message) ; enters at execute2
)

(event Custom|CustomEvent_3
  (params (AddressPattern :type OSC%20Address%20Structure%20%28by%20ref%29) (Message :type OSC%20Message%20Structure%20%28by%20ref%29) (IPAddress :type String) (Port :type Integer))
  (|OSCControl_3 "lvl1/cube1/scale" (delegate Custom|CustomEvent_3) Message) ; enters at execute2
)

(event Custom|OSC%20Event%20Camera%202
  (params (AddressPattern :type OSC%20Address%20Structure%20%28by%20ref%29) (Message :type OSC%20Message%20Structure%20%28by%20ref%29) (IPAddress :type String) (Port :type Integer))
  (|OSCOSCControl_Cam_2 "scene1/cam2" (delegate Custom|OSC%20Event%20Camera%202) Message) ; enters at execute2
)

(event Custom|CustomEvent_4
  (params (AddressPattern :type OSC%20Address%20Structure%20%28by%20ref%29) (Message :type OSC%20Message%20Structure%20%28by%20ref%29) (IPAddress :type String) (Port :type Integer))
  (|OSCControl_3_2 "lvl1/cube1/pos/z" (delegate Custom|CustomEvent_4) Message) ; enters at execute2
)

(event Custom|CustomEvent_6
  (params (AddressPattern :type OSC%20Address%20Structure%20%28by%20ref%29) (Message :type OSC%20Message%20Structure%20%28by%20ref%29) (IPAddress :type String) (Port :type Integer))
  (|OSCControl_Audio "scene1/audio" (delegate Custom|CustomEvent_6) Message) ; enters at execute2
)

(event Custom|CustomEvent_7
  (params (AddressPattern :type OSC%20Address%20Structure%20%28by%20ref%29) (Message :type OSC%20Message%20Structure%20%28by%20ref%29) (IPAddress :type String) (Port :type Integer))
  (|OSCControl_Sky "scene1/sky/absorption_scale" (delegate Custom|CustomEvent_7) Message) ; enters at execute2
)

(event Custom|CustomEvent_9
  (params (AddressPattern :type OSC%20Address%20Structure%20%28by%20ref%29) (Message :type OSC%20Message%20Structure%20%28by%20ref%29) (IPAddress :type String) (Port :type Integer))
  (|OSCControl_Sky_3 "scene1/directional_light_world/intensity" (delegate Custom|CustomEvent_9) Message) ; enters at execute2
)

(event Custom|OSC%20ProstProcessing
  (params (AddressPattern :type OSC%20Address%20Structure%20%28by%20ref%29) (Message :type OSC%20Message%20Structure%20%28by%20ref%29) (IPAddress :type String) (Port :type Integer))
  (|OSCControl_PostProcessing "scene1/fx/bloom" (delegate Custom|OSC%20ProstProcessing) Message) ; enters at execute2
)

(event Custom|CustomEvent_2
  (params (AddressPattern :type OSC%20Address%20Structure%20%28by%20ref%29) (Message :type OSC%20Message%20Structure%20%28by%20ref%29) (IPAddress :type String) (Port :type Integer))
  (|OSCControl_2_2_2 "lvl1/light1/b" (delegate Custom|CustomEvent_2) Message) ; enters at execute2
)

(event Custom|OSC%20ProstProcessing%202
  (params (AddressPattern :type OSC%20Address%20Structure%20%28by%20ref%29) (Message :type OSC%20Message%20Structure%20%28by%20ref%29) (IPAddress :type String) (Port :type Integer))
  (|OSCControl_PostProcessing_2 "scene1/fx/chromatic" (delegate Custom|OSC%20ProstProcessing%202) Message) ; enters at execute2
)

(event Custom|OSC%20ProstProcessing%203
  (params (AddressPattern :type OSC%20Address%20Structure%20%28by%20ref%29) (Message :type OSC%20Message%20Structure%20%28by%20ref%29) (IPAddress :type String) (Port :type Integer))
  (|OSCControl_PostProcessing_2_2 "scene1/fx/vignette" (delegate Custom|OSC%20ProstProcessing%203) Message) ; enters at execute2
)

(event Custom|CustomEvent_8
  (params (AddressPattern :type OSC%20Address%20Structure%20%28by%20ref%29) (Message :type OSC%20Message%20Structure%20%28by%20ref%29) (IPAddress :type String) (Port :type Integer))
  (|OSCControl_Sky_2 "scene1/sky/intensity" (delegate Custom|CustomEvent_8) Message) ; enters at execute2
)

(event Custom|OSC%20ProstProcessing%204
  (params (AddressPattern :type OSC%20Address%20Structure%20%28by%20ref%29) (Message :type OSC%20Message%20Structure%20%28by%20ref%29) (IPAddress :type String) (Port :type Integer))
  (|OSCControl_PostProcessing_2_2_2 "scene1/fx/noise" (delegate Custom|OSC%20ProstProcessing%204) Message) ; enters at execute2
)

(event Custom|CustomEvent
  (params (AddressPattern :type OSC%20Address%20Structure%20%28by%20ref%29) (Message :type OSC%20Message%20Structure%20%28by%20ref%29) (IPAddress :type String) (Port :type Integer))
  (|OSCControl_2 "lvl1/light1/r" (delegate Custom|CustomEvent) Message) ; enters at execute2
)

(event Custom|OSC%20Event%20Camera%20Player
  (params (AddressPattern :type OSC%20Address%20Structure%20%28by%20ref%29) (Message :type OSC%20Message%20Structure%20%28by%20ref%29) (IPAddress :type String) (Port :type Integer))
  (|OSCControl_Cam "scene1/cam_player" (delegate Custom|OSC%20Event%20Camera%20Player) Message) ; enters at execute2
)

(event Custom|CustomEvent_11
  (params (AddressPattern :type OSC%20Address%20Structure%20%28by%20ref%29) (Message :type OSC%20Message%20Structure%20%28by%20ref%29) (IPAddress :type String) (Port :type Integer))
  (|OSCControl_Audio_2 "scene1/react" (delegate Custom|CustomEvent_11) Message) ; enters at execute2
)

(event Custom|CustomEvent_1
  (params (AddressPattern :type OSC%20Address%20Structure%20%28by%20ref%29) (Message :type OSC%20Message%20Structure%20%28by%20ref%29) (IPAddress :type String) (Port :type Integer))
  (|OSCControl_2_2 "lvl1/light1/g" (delegate Custom|CustomEvent_1) Message) ; enters at execute2
)

(event Custom|OSC%20Event%20Camera%201
  (params (AddressPattern :type OSC%20Address%20Structure%20%28by%20ref%29) (Message :type OSC%20Message%20Structure%20%28by%20ref%29) (IPAddress :type String) (Port :type Integer))
  (|OSCOSCControl_Cam_1 "scene1/cam1" (delegate Custom|OSC%20Event%20Camera%201) Message) ; enters at execute2
)

(event Custom|OnMsgReceived_AddressPattern
  (params (AddressPattern :type OSC%20Address%20Structure%20%28by%20ref%29) (Message :type OSC%20Message%20Structure%20%28by%20ref%29) (IPAddress :type String) (Port :type Integer))
  (|OSCControl "lvl1/light1/intensity" (delegate Custom|OnMsgReceived_AddressPattern) Message) ; enters at execute2
)

(event Custom|CustomEvent_5
  (params (AddressPattern :type OSC%20Address%20Structure%20%28by%20ref%29) (Message :type OSC%20Message%20Structure%20%28by%20ref%29) (IPAddress :type String) (Port :type Integer))
  (|OSCControl_3_2_2 "lvl/change" (delegate Custom|CustomEvent_5) Message) ; enters at execute2
)

(event EventBeginPlay
  (Utilities|FlowControl|Sequence
    (:then_0
      ;[1 1 1] Binding to Any Message
      (bind _returnvalue (Class|OSCManager|CreateOSCServer "127.0.0.1" 7000 false true "" 0))
      (bind _output_get (Variables|Default|SetOSC%20SERVER _returnvalue))
      (EventDispatchers|AssignOnOscMessageReceived _output_get (delegate Custom|OnMsgReceived))
      (Utilities|FlowControl|DoOnce false) ; enters at Reset
    )))

(event EventTick
  (params (DeltaSeconds :type Float%20%28single-precision%29))
  (bind _returnvalue (Game|GetPlayerController 0))
  (bind _osc_postprocessing (Variables|Default|GetOSC%20PostProcessing))
  (bind _settings (Variables|/Script/Engine.PostProcessVolume|GetSettings _osc_postprocessing))
  (Utilities|IsValid (stale _returnvalue_2)
    (:Is%20Valid
      (Utilities|FlowControl|Sequence
        (:then_0
          (bind _value (|OSCControl "lvl1/light1/intensity" (delegate Custom|OnMsgReceived_AddressPattern) (stale Custom|OnMsgReceived_AddressPattern Message)))
          (bind _aspoint_light (Utilities|Casting|CastToPointLight (Variables|Default|GetOSC%20Light)))
          (Rendering|Components|Light|SetIntensity (Variables|/Script/Engine.Light|GetLightComponent _aspoint_light) _value))
        (:then_1
          (Utilities|FlowControl|Sequence
            (:then_0
              (bind _value_2 (|OSCControl_2 "lvl1/light1/r" (delegate Custom|CustomEvent) (stale Custom|CustomEvent Message))))
            (:then_1
              (bind _value_3 (|OSCControl_2_2 "lvl1/light1/g" (delegate Custom|CustomEvent_1) (stale Custom|CustomEvent_1 Message))))
            (:then_2
              (bind _value_4 (|OSCControl_2_2_2 "lvl1/light1/b" (delegate Custom|CustomEvent_2) (stale Custom|CustomEvent_2 Message)))))
          (bind _aspoint_light_2 (Utilities|Casting|CastToPointLight (Variables|Default|GetOSC%20Light)))
          (Rendering|Components|Light|SetLightColor (Variables|/Script/Engine.Light|GetLightComponent _aspoint_light_2) (Utilities|Struct|MakeLinearColor _value_2 _value_3 _value_4 0.0) true))
        (:then_2
          (bind _value_5 (|OSCControl_3 "lvl1/cube1/scale" (delegate Custom|CustomEvent_3) (stale Custom|CustomEvent_3 Message)))
          (Transformation|SetActorScale3D (Variables|Default|GetOSC%20Cube) (Math|Vector|MakeVector _value_5 _value_5 _value_5)))
        (:then_3
          (bind _value_6 (|OSCControl_3_2 "lvl1/cube1/pos/z" (delegate Custom|CustomEvent_4) (stale Custom|CustomEvent_4 Message)))
          (Transformation|SetActorLocation (Variables|Default|GetOSC%20Cube) (Math|Vector|MakeVector 0.0 0.0 _value_6) false false))
        (:then_4
          (bind _value_7 (|OSCControl_3_2_2 "lvl/change" (delegate Custom|CustomEvent_5) (stale Custom|CustomEvent_5 Message)))
          (if (== _value_7 1.0)
            (Class|GameplayStatics|LoadStreamLevelbySoftObjectPtr "/Game/Maps/Level_Streaming_Test.Level_Streaming_Test" true false)
            (else
              (Class|GameplayStatics|UnloadStreamLevelbySoftObjectPtr "/Game/Maps/Level_Streaming_Test.Level_Streaming_Test" false))))
        (:then_5
          (bind _value_8 (|OSCControl_Audio "scene1/audio" (delegate Custom|CustomEvent_6) (stale Custom|CustomEvent_6 Message)))
          (if (== _value_8 1.0)
            _
            (else
              _))
          (bind _ascapture_lr (Utilities|Casting|CastTocaptureLR (Variables|Default|GetOSC%20Audio%20Capture)))
          (bind _output_get (Variables|/Game/Blueprints/captureLR.captureLR_C|SetAudioToggle _ascapture_lr (== _value_8 1.0)))
          (Development|PrintString (Utilities|String|ToString(Boolean) _output_get) false))
        (:then_6
          (Utilities|FlowControl|Sequence
            (:then_0
              (bind _value_9 (|OSCControl_Sky "scene1/sky/absorption_scale" (delegate Custom|CustomEvent_7) (stale Custom|CustomEvent_7 Message)))
              (Class|SkyAtmosphereComponent|SetMieAbsorptionScale (Variables|/SunPosition/SunSky.SunSky_C|GetSkyAtmosphere (Variables|Default|GetOSC%20SunSky)) _value_9))
            (:then_1
              (bind _value_10 (|OSCControl_Sky_2 "scene1/sky/intensity" (delegate Custom|CustomEvent_8) (stale Custom|CustomEvent_8 Message)))
              (Rendering|Components|Light|SetIntensity (Variables|/SunPosition/SunSky.SunSky_C|GetDirectionalLight (Variables|Default|GetOSC%20SunSky)) _value_10))
            (:then_2
              (bind _value_11 (|OSCControl_Sky_3 "scene1/directional_light_world/intensity" (delegate Custom|CustomEvent_9) (stale Custom|CustomEvent_9 Message)))
              (Rendering|Components|Light|SetIntensity (Variables|/Script/Engine.Light|GetLightComponent (Variables|Default|GetOSC%20DirectionalLightWorld)) _value_11))))
        (:then_7
          (Utilities|FlowControl|Sequence
            (:then_0
              (bind _value_12 (|OSCControl_PostProcessing "scene1/fx/bloom" (delegate Custom|OSC%20ProstProcessing) (stale Custom|OSC%20ProstProcessing Message)))
              (Utilities|Struct|SetmembersinPostProcessSettings _settings _value_12))
            (:then_1
              (bind _value_13 (|OSCControl_PostProcessing_2 "scene1/fx/chromatic" (delegate Custom|OSC%20ProstProcessing%202) (stale Custom|OSC%20ProstProcessing%202 Message)))
              (Utilities|Struct|SetmembersinPostProcessSettings _settings _value_13))
            (:then_2
              (bind _value_14 (|OSCControl_PostProcessing_2_2 "scene1/fx/vignette" (delegate Custom|OSC%20ProstProcessing%203) (stale Custom|OSC%20ProstProcessing%203 Message)))
              (Utilities|Struct|SetmembersinPostProcessSettings _settings _value_14))
            (:then_3
              (bind _value_15 (|OSCControl_PostProcessing_2_2_2 "scene1/fx/noise" (delegate Custom|OSC%20ProstProcessing%204) (stale Custom|OSC%20ProstProcessing%204 Message)))
              (Utilities|Struct|SetmembersinPostProcessSettings _settings _value_15))))
        (:then_8
          (Utilities|FlowControl|Sequence
            (:then_0
              (|OSCControl_Cam "scene1/cam_player" (delegate Custom|OSC%20Event%20Camera%20Player) (stale Custom|OSC%20Event%20Camera%20Player Message))
              (Game|Player|SetViewTargetwithBlend _returnvalue 0 (Variables|Default|GetOSC%20Camera%20Speed) "VTBlend_EaseInOut" 1.0 false))
            (:then_1
              (|OSCOSCControl_Cam_1 "scene1/cam1" (delegate Custom|OSC%20Event%20Camera%201) (stale Custom|OSC%20Event%20Camera%201 Message))
              (Game|Player|SetViewTargetwithBlend _returnvalue (Variables|Default|GetOSC%20Camera%201) (Variables|Default|GetOSC%20Camera%20Speed) "VTBlend_EaseInOut" 1.0 false))
            (:then_2
              (|OSCOSCControl_Cam_2 "scene1/cam2" (delegate Custom|OSC%20Event%20Camera%202) (stale Custom|OSC%20Event%20Camera%202 Message))
              (Game|Player|SetViewTargetwithBlend _returnvalue (Variables|Default|GetOSC%20Camera%202) (Variables|Default|GetOSC%20Camera%20Speed) "VTBlend_EaseInOut" 1.0 false))
            (:then_3
              (bind _value_16 (|OSCOSCControl_Cam_2_2 "scene1/camera/speed" (delegate Custom|CustomEvent_10) (stale Custom|CustomEvent_10 Message)))
              (Variables|Default|SetOSC%20Camera%20Speed _value_16))))
        (:then_9
          (bind _value_17 (|OSCControl_Audio_2 "scene1/react" (delegate Custom|CustomEvent_11) (stale Custom|CustomEvent_11 Message)))
          (bind _ascapture_lr_2 (Utilities|Casting|CastTocaptureLR (Variables|Default|GetOSC%20Audio%20Capture)))
          (bind _output_get_2 (Variables|/Game/Blueprints/captureLR.captureLR_C|SetAudioReactivity _ascapture_lr_2 _value_17))
          (Development|PrintString (Utilities|String|ToString(Float) _output_get_2)))))
    (:Is%20Not%20Valid
      (Utilities|FlowControl|DoOnce false :!label _label
        (:Completed
          ;[1 1 1] Binding to Any Message
          (bind _returnvalue_2 (Class|OSCManager|CreateOSCServer "127.0.0.1" 7000 false true "" 0))
          (bind _output_get_3 (Variables|Default|SetOSC%20SERVER _returnvalue_2))
          (EventDispatchers|AssignOnOscMessageReceived _output_get_3 (delegate Custom|OnMsgReceived))
          (goto _label Reset))))))

(fn ConstructionScript)