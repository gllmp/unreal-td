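; An actor that visualizes live audio capture loudness through a text readout and a moving sphere.
; The AudioCapture envelope callback scales the value, logs it, shows it on the TextRender and drives the Sphere's relative Z height.
; Each Tick, VolumeValue takes the envelope value while AudioToggle is on and drops to zero otherwise, though nothing in this graph reads it.
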(event OnAudioEnvelopeValue(AudioCapture)
  (params (EnvelopeValue :type Float%20%28single-precision%29))
  (bind _returnvalue (* EnvelopeValue 1e+02))
  (Development|PrintString (Utilities|String|ToString(Float) _returnvalue) false)
  (Rendering|Components|TextRender|SetText (Variables|Default|GetTextRender) (Utilities|Text|ToText(Float) _returnvalue "HalfToEven"))
  (Transformation|SetRelativeLocation (Variables|Default|GetSphere) (Math|Vector|MakeVector 0.0 0.0 (* _returnvalue 5.0)) false false))

(event EventTick
  (params (DeltaSeconds :type Float%20%28single-precision%29))
  (if (== (Variables|Default|GetAudioToggle) true)
    (Variables|Default|SetVolumeValue (stale OnAudioEnvelopeValue(AudioCapture) EnvelopeValue))
    (else
      (Variables|Default|SetVolumeValue 0.0))))

(fn ConstructionScript)